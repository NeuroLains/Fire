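; Moving actor that carries component H back and forth along the Track spline, spinning it as it travels and pausing at each end.
; Tick advances a clamped MovementTime, which MovementCurve remaps to a spline location, and reverses direction after either limit.
; While moving, a sphere trace at component F leaves a short-lived debug trail, with its hits unused.
; The construction script sets the spline duration and previews StartPosition.
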(event EventBeginPlay)

(event EventTick
  (params (DeltaSeconds :type Float%20%28single-precision%29))
  (bind _f (Variables|Default|GetF))
  (bind _returnvalue (Transformation|GetWorldLocation _f))
  (Variables|Default|SetDeltaSeconds DeltaSeconds)
  (if (Variables|Default|GetCanMove)
    (Transformation|AddLocalRotation (Variables|Default|GetH) (Math|Rotator|MakeRotator (Variables|Default|GetRotateX) (Variables|Default|GetRotateY) (Variables|Default|GetRotateZ)) false false)
    (Collision|MultiSphereTraceByChannel _returnvalue _returnvalue 1e+01 "TraceTypeQuery1" false 0 "ForDuration" true "(R=1.000000,G=1.000000,B=1.000000,A=1.000000)" "(R=0.000000,G=1.000000,B=0.000000,A=1.000000)" 1.5)
    (Variables|Default|SetMovementTime (Math|Float|Clamp(Float) (+ (Variables|Default|GetMovementTime) (* (Variables|Default|GetMovementDirection) (Variables|Default|GetDeltaSeconds))) 0.0 (Variables|/Script/Engine.SplineComponent|GetDuration (Variables|Default|GetTrack))))
    (Math|Integer|CompareInt (Variables|Default|GetMovementDirection)
      (:>
        (if (Math|Float|NearlyEqual(Float) (Variables|/Script/Engine.SplineComponent|GetDuration (Variables|Default|GetTrack)) (Variables|Default|GetMovementTime) 1e-06)
          (Variables|Default|SetCanMove false :!label _label)
          (Variables|Default|SetMovementDirection (* (Variables|Default|GetMovementDirection) -1))
          (Utilities|FlowControl|Delay (Variables|Default|GetWaitTime))
          (Variables|Default|SetCanMove true)
          (else
            (CallFunction|UpdateObjectLocation :!label _label_2))))
      (:<
        (if (Math|Float|NearlyEqual(Float) 0.0 (Variables|Default|GetMovementTime) 1e-06)
          (goto _label)
          (else
            (goto _label_2)))))))

(event Collision|EventActorBeginOverlap
  (params (OtherActor :type Actor%20Object%20Reference)))

(fn ConstructionScript
  (Variables|/Script/Engine.SplineComponent|SetDuration (Variables|Default|GetTrack) (Variables|Default|GetMovementDuration))
  (Variables|Default|SetMovementTime (* (Variables|Default|GetMovementDuration) (Variables|Default|GetStartPosition)))
  (CallFunction|UpdateObjectLocation))

(fn UpdateObjectLocation
  (bind _track (Variables|Default|GetTrack))
  (bind _duration (Variables|/Script/Engine.SplineComponent|GetDuration _track))
  (Transformation|SetWorldLocation (Variables|Default|GetH) (Spline|GetLocationatTime (Variables|Default|GetTrack) (Math|Float|MapRangeClamped (Math|Curves|GetFloatValue (Variables|Default|GetMovementCurve) (Math|Float|NormalizetoRange (Variables|Default|GetMovementTime) 0.0 _duration)) 0.0 1.0 0.0 _duration) "World" false) false false))